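; Player controller that tracks whether the player is using a gamepad, through an IsUsingGamepad flag.
; Any key press sets the flag according to whether the key is a gamepad key.
; Tick also clears it when an input axis reads non-zero or, while the GameInstance's SelectionWheel is valid, when the mouse is away from the DPI-scaled viewport center.
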(event EventBeginPlay)

(event EventTick
  (params (DeltaSeconds :type Float%20%28single-precision%29))
  (bind _returnvalue (Viewport|GetViewportSize))
  (bind _returnvalue_2 (Class|WidgetLayoutLibrary|GetViewportScale))
  (Variables|/Game/ReworkerBP/MyGameInstance.MyGameInstance_C|GetSelectionWheel (.AsMy%20Game%20Instance (Utilities|Casting|CastToMyGameInstance (Game|GetGameInstance)))
    (:then
      ;[1 1 1] Using mouse in wheel
      (bind _returnvalue_3 (Class|WidgetLayoutLibrary|GetMousePositiononViewport))
      (if (Math|Vector|NotEqual(Vector) _returnvalue_3 (/ (Math|Vector2D|MakeVector2D (/ (.x _returnvalue) _returnvalue_2) (/ (.y _returnvalue) _returnvalue_2)) 2.0) 0.1)
        (Variables|Default|SetIsUsingGamepad false :!label _label)))
    (:else
      (if (or (!= (Class|Actor|GetInputAxisKeyValue) 0.0) (!= (Class|Actor|GetInputAxisKeyValue) 0.0))
        (goto _label)))))

(event Input|KeyboardEvents|AnyKey
  (params (Key :type Key%20Structure :default "None"))
  (:Pressed
    (if (Class|KismetInputLibrary|KeyIsGamepadKey Key)
      (Variables|Default|SetIsUsingGamepad true)
      (else
        (Variables|Default|SetIsUsingGamepad false)))))

(fn ConstructionScript)