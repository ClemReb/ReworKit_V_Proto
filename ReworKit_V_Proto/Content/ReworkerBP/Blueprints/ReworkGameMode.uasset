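; Game mode that respawns the player's Reworker character when it is destroyed.
; On BeginPlay it binds to the character's destroyed event; on death it spawns a new Reworker at a stored spawn location, possesses it and rebinds.
; It then adds a new HUD widget, restores skill slots and equipped movement abilities from saved GameInstance values, and refreshes the character's modulation.
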(event Custom|OnDeath
  (params (DestroyedActor :type Actor%20Object%20Reference))
  (bind _returnvalue (Game|GetPlayerController 0))
  (bind _returnvalue_2 (Game|GetPlayerCharacter 0))
  (bind _asreworker (Utilities|Casting|CastToReworker _returnvalue_2))
  (bind _returnvalue_3 (Game|SpawnActorfromClass "/Game/ReworkerBP/Blueprints/Reworker.Reworker_C" (Variables|Default|GetSpawnLocation) "AdjustIfPossibleButAlwaysSpawn" 0 0))
  (Pawn|Possess _returnvalue _returnvalue_3)
  (CallFunction|Respawn)
  (bind _returnvalue_4 (UserInterface|CreateWidget "/Game/HUD/HUD_V2/IG_HUD_V2.IG_HUD_V2_C" _returnvalue))
  (UserInterface|Viewport|AddtoViewport _returnvalue_4 0)
  (|ResetSkills)
  (Default|ModulationRefresh _asreworker)
  (Default|ModulationRefresh _asreworker))

(event Custom|Respawn
  (bind _asreworker (Utilities|Casting|CastToReworker (Game|GetPlayerCharacter 0)))
  (Game|BindEventtoOnDestroyed _asreworker (delegate Custom|OnDeath)))

(event EventBeginPlay
  (bind _asreworker (Utilities|Casting|CastToReworker (Game|GetPlayerCharacter 0)))
  (Game|BindEventtoOnDestroyed _asreworker (delegate Custom|OnDeath)))

(fn ConstructionScript)